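; Base decal Blueprint for the Impact Effect System that gives decals a varied appearance.
; On BeginPlay it sets the decal to a random material from PossibleDecalMaterials and, when ShouldRandomizeRotation is enabled, randomizes its roll while keeping pitch and yaw.
; An empty array or invalid pick prints an on-screen warning naming the object and leaves the default material in place.
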(event EventBeginPlay
  (bind _material (CallFunction|RandomDecalMaterial))
  ;[0.9922 1 0] IES uses custom decal blueprints,
  ; it allows to easily setup randomized decals, with random rotation and material
  (Utilities|FlowControl|Sequence
    (:then_0
      (Utilities|IsValid _material
        (:Is%20Valid
          (Rendering|Components|Decal|SetDecalMaterial (Variables|Default|GetDecal) _material) ; Set random material from PossibleDecalMaterials array
        )))
    (:then_1
      (if (Variables|Default|GetShouldRandomizeRotation)
        (CallFunction|RandomizeRotation (Variables|Default|GetDecal)) ; set random ROLL value
      ))))

(fn ConstructionScript)

(fn RandomDecalMaterial
  (bind _possibledecalmaterials (Variables|Default|GetPossibleDecalMaterials))
  (bind _returnvalue (Utilities|Array|Length _possibledecalmaterials))
  (if (> _returnvalue 0) ; Check if array is not empty
    (bind _output_get (LocalVariables|SetRandomizedMaterial (Utilities|Array|Get(acopy) _possibledecalmaterials (Math|Random|RandomInteger _returnvalue))))
    (Utilities|IsValid _output_get ; check if randomized item is valid
      (:Is%20Valid
        (return (LocalVariables|GetRandomizedMaterial)) ; Success
      )
      (:Is%20Not%20Valid
        (Development|PrintString (Utilities|String|Append "! IES WARNING ! 
There's at least one empty item in PossibleMaterials array in \"" (Utilities|GetDisplayName self) "\"") true true "(R=1.000000,G=0.846693,B=0.000000,A=1.000000)" 15.0)))
    (else
      (Development|PrintString (Utilities|String|Append "! IES WARNING ! 
PossibleMaterials array for \"" (Utilities|GetDisplayName self) "\" is empty! 
Leaving default material") true true "(R=1.000000,G=0.846693,B=0.000000,A=1.000000)" 15.0)))
  (return 0) ; array is not valid
)

(fn RandomizeRotation
  (params (Target :type Scene%20Component%20Object%20Reference))
  (bind _relativerotation (Variables|/Script/Engine.SceneComponent|GetRelativeRotation Target))
  (Transformation|SetRelativeRotation Target (Math|Rotator|MakeRotator (Math|Random|RandomFloatinRange 0.0 3.6e+02) (.pitch _relativerotation) (.yaw _relativerotation)) false false) ; randomize ROLL rotation for different apperance
)