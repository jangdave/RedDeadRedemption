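; Impact effect system base Blueprint for physical objects that play impact effects when their owner hits something.
; It extends a parent impact component's owner hit event, forwarding the hit only when the owner's speed exceeds a minimum velocity and no cooldown is active.
; The velocity and cooldown gate prevents effect spam from small or repeated contacts.
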(event EventOwnerHitEvent
  (params (SelfActor :type Actor%20Object%20Reference) (OtherActor :type Actor%20Object%20Reference) (NormalImpulse :type Vector :default "0, 0, 0") (Hit :type Hit%20Result%20Structure%20%28by%20ref%29))
  ;[0.1719 0 1] Check velocity condition
  (if (and (> (Math|Vector|VectorLength (Transformation|GetVelocity SelfActor)) (Variables|Setup|GetEffectMinimumVelocity)) (not (Variables|Default|GetCooldown))) ; Check If Velocity is big enough, to prevent effects spam
    (|CallParentFunction SelfActor OtherActor NormalImpulse Hit)))

(event EventBeginPlay
  (|CallParentFunction))