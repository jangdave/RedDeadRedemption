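; Impact Effect System component that spawns sound, particle and decal effects based on the physical material its owner hits.
; On BeginPlay it builds a material-to-effect map from a data table, warning about bad rows, and binds to the owner's hit event.
; Hits pass enable, owner-collision and cooldown checks, then matched effects attach to the hit component, optionally falling back to the first map entry.
; Optional debug drawing shows hit details.
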(event Custom|OwnerHitEvent
  (params (SelfActor :type Actor%20Object%20Reference) (OtherActor :type Actor%20Object%20Reference) (NormalImpulse :type Vector) (Hit :type Hit%20Result%20Structure%20%28by%20ref%29))
  ;[0 0.3672 1] Binded hit Event
  (if (Variables|Private|GetIESEnabled) ; Is IES disabled externally
    (CallFunction|SpawnEffectEvent Hit OtherActor)))

(event Custom|SpawnEffectEvent
  (params (HitInfo :type Hit%20Result%20Structure) (HitActor :type Actor%20Object%20Reference))
  (bind _effectbyhit (Variables|Private|GetEffectByHit))
  (bind (_physmaterial _sound _particle _decal) (Utilities|Struct|BreakIES_BaseStruct _effectbyhit))
  ;[0 0.2512 0.5701] Find and Spawn Effect After Hit
  (Variables|Private|SetLastHitInfo HitInfo)
  (if (not (and (not (Variables|Setup|GetEffectOnCollideWithOwner)) (== HitActor (Variables|Public|GetOwnerActor))))
    (if (not (Variables|Public|GetCooldown)) ; If cooldown ended
      (Utilities|FlowControl|Sequence
        (:then_0
          (Utilities|DEBUGMacro) ; handle debug
        )
        (:then_1
          (Variables|Public|SetCooldown true) ; Handle Cooldown
          (Utilities|FlowControl|Delay (Variables|Setup|GetEffectSpawnCooldown))
          (Variables|Public|SetCooldown false))
        (:then_2
          (Private|SetEffectbyMat) ; Find material in Effects Map based on Phys Material that was hit
        )
        (:then_3
          (Utilities|IsValid _physmaterial ; if effect is set
            (:Is%20Valid
              (Private|SpawnSound _sound)
              (Private|SpawnParticle _particle)
              (Private|SpawnDecal _decal))))))))

(event EventBeginPlay
  ;[0 0.06764 0.7537] Bind Event on begin play - On Owner hit
  (Private|SetEffectsfromSetup) ; Create Effects Map, to have easy access to effects by given physical material
  (bind _output_get (Variables|Public|SetOwnerActor (Components|GetOwner)))
  (Collision|BindEventtoOnActorHit _output_get (delegate Custom|OwnerHitEvent)) ; Bind to hit event
)

(fn SpawnSound
  (params (Sound :type Sound%20Base%20Object%20Reference))
  (bind _lasthitinfo (Variables|Private|GetLastHitInfo))
  (bind (_bblockinghit _binitialoverlap _time _distance _location _impactpoint _normal _impactnormal _physmat _hitactor _hitcomponent) (Collision|BreakHitResult _lasthitinfo))
  (Utilities|IsValid Sound
    (:Is%20Valid
      (Audio|SpawnSoundAttached Sound _hitcomponent "None" _location (Math|Rotator|MakeRotfromX _impactnormal) "KeepWorldPosition" true 1.0 1.0 0.0 0 0))))

(fn SpawnParticle
  (params (Particle :type Particle%20System%20Object%20Reference))
  (bind _lasthitinfo (Variables|Private|GetLastHitInfo))
  (bind (_bblockinghit _binitialoverlap _time _distance _location _impactpoint _normal _impactnormal _physmat _hitactor _hitcomponent _hitbonename) (Collision|BreakHitResult _lasthitinfo))
  (Utilities|IsValid Particle
    (:Is%20Valid
      (Effects|SpawnEmitterAttached Particle _hitcomponent _hitbonename _impactpoint (Math|Rotator|MakeRotfromX _impactnormal) "1.000000,1.000000,1.000000" "KeepWorldPosition"))))

(fn SpawnDecal
  (params (Decal :type BP%20IES%20Decal%20Base%20Class%20Reference))
  (bind _lasthitinfo (Variables|Private|GetLastHitInfo))
  (bind (_bblockinghit _binitialoverlap _time _distance _location _impactpoint _normal _impactnormal _physmat _hitactor _hitcomponent _hitbonename) (Collision|BreakHitResult _lasthitinfo))
  (if (Utilities|IsValidClass Decal)
    (bind _returnvalue (Game|SpawnActorfromClass Decal (Math|Transform|MakeTransform _impactpoint (Math|Rotator|MakeRotfromX _impactnormal)) "Undefined" 0 0))
    (Transformation|AttachComponentToComponent _returnvalue _hitcomponent _hitbonename "KeepWorld" "KeepWorld" "KeepWorld" true)))

(fn SetEffectbyMat
  (bind _effects (Variables|Public|GetEffects))
  (bind _lasthitinfo (Variables|Private|GetLastHitInfo))
  (bind _physmat (Collision|BreakHitResult _lasthitinfo))
  (bind (_value _returnvalue) (Utilities|Map|Find _effects _physmat))
  (if _returnvalue
    (Variables|Private|SetEffectByHit _value)
    (return)
    (else
      ;[0 0.3285 0.4928] If physical material was not found in EffectsDataTable, should spawn first item of Effects map?
      (if (Variables|Setup|GetAlwaysSpawnSomething)
        (bind _values (Utilities|Map|Values (Variables|Public|GetEffects)))
        (Variables|Private|SetEffectByHit (Utilities|Array|Get(acopy) _values))
        (return)))))

(fn SetEffectsfromSetup
  (bind _effectsdatatable (Variables|Setup|GetEffectsDataTable))
  (bind _effects (Variables|Public|GetEffects))
  (Utilities|Map|Clear (Variables|Public|GetEffects))
  (Utilities|IsValid _effectsdatatable
    (:Is%20Valid
      (bind _outrownames (DataTable|GetDataTableRowNames _effectsdatatable))
      (for _array_element _outrownames
        (bind _returnvalue (Utilities|GetDataTableRow (Variables|Setup|GetEffectsDataTable) _array_element)
          (:then
            (Utilities|IsValid (.PhysMaterial (Utilities|Struct|BreakIES_BaseStruct _returnvalue)) ; check if physical material is assigned in Setup row
              (:Is%20Valid
                (if (Utilities|Map|Contains _effects (.PhysMaterial (Utilities|Struct|BreakIES_BaseStruct _returnvalue))) ; check if Physical Material is Unique
                  (Development|PrintString (Utilities|String|Append "--- IES WARNING ! 
" (Utilities|GetDisplayName self) " hasData Table with same PhysicalMaterial in different rows!" " 
Row name: " (Utilities|String|ToString(Name) _array_element)) true true "(R=0.468750,G=0.007992,B=0.000000,A=1.000000)" 1e+01)
                  (else
                    (Utilities|Map|Add _effects (.PhysMaterial (Utilities|Struct|BreakIES_BaseStruct _returnvalue)) (Utilities|Struct|MakeIES_BaseStruct (.PhysMaterial (Utilities|Struct|BreakIES_BaseStruct _returnvalue)) (.Sound (Utilities|Struct|BreakIES_BaseStruct _returnvalue)) (.Particle (Utilities|Struct|BreakIES_BaseStruct _returnvalue)) (.Decal (Utilities|Struct|BreakIES_BaseStruct _returnvalue)))))))
              (:Is%20Not%20Valid
                (Development|PrintString (Utilities|String|Append "--- IES WARNING ! 
" (Utilities|GetDisplayName self) " has IES Setup Data Table with empty PhysicalMaterial variable!" " 
Row name: " (Utilities|String|ToString(Name) _array_element)) true true "(R=0.468750,G=0.007992,B=0.000000,A=1.000000)" 1e+01)))))))
    (:Is%20Not%20Valid
      (Development|PrintString (Utilities|String|Append (Utilities|GetDisplayName self) " has IES comp but empty EffectsDataTable !") true true "(R=0.000000,G=0.468750,B=0.049201,A=1.000000)" 5.0))))

(fn SetEnableIES
  (params (New%20Enable :type Boolean))
  (Variables|Private|SetIESEnabled New%20Enable))