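; BP_Horse is a rideable horse that the player controller possesses in place of the player character.
; HorseRiding stores the character as Rider, possesses the horse and shows PlayerMesh, apparently a stand-in rider.
; The overlap events are empty.
; Unconnected logic would bind HorseRiding to a BP_RedPlayer event and dismount by moving Rider to DetachComp, repossessing it and hiding PlayerMesh, but never runs.
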(event OnComponentBeginOverlap(boxComp)
  (params (OverlappedComponent :type Primitive%20Component%20Object%20Reference) (OtherActor :type Actor%20Object%20Reference) (OtherComp :type Primitive%20Component%20Object%20Reference) (OtherBodyIndex :type Integer) (bFromSweep :type Boolean) (SweepResult :type Hit%20Result%20Structure%20%28by%20ref%29)))

(event OnComponentEndOverlap(boxComp)
  (params (OverlappedComponent :type Primitive%20Component%20Object%20Reference) (OtherActor :type Actor%20Object%20Reference) (OtherComp :type Primitive%20Component%20Object%20Reference) (OtherBodyIndex :type Integer)))

(event Custom|HorseRiding
  (Variables|Default|SetRider (Game|GetPlayerCharacter 0))
  (Pawn|Possess (Game|GetPlayerController 0) self)
  (Rendering|SetVisibility (Variables|Default|GetplayerMesh) true false))

(event EventBeginPlay)

(event Collision|EventActorBeginOverlap
  (params (OtherActor :type Actor%20Object%20Reference)))

(event EventTick
  (params (DeltaSeconds :type Float%20%28single-precision%29)))

(event Input|ActionEvents|InputActionHorseRide
  (params (Key :type Key%20Structure :default "None")))

(fn ConstructionScript)